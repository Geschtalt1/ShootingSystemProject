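; BP_PlayerCharacter is the player-controlled character handling movement, camera look and weapon input.
; On possession by a PlayerController it adds the IMC_Default Enhanced Input mapping context.
; Move and look actions drive movement input and controller yaw and pitch.
; Fire, fire-mode and reload actions forward interface messages to the weapon held in the WeaponActor child actor component, keeping weapon logic out of the character.
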(event `EnhancedInput|/Game/Core/Data/Input/Action/IA_Move`
  (params (ActionValue :type "Vector2D Structure") (ElapsedSeconds :type "Float (double-precision)") (TriggeredSeconds :type "Float (double-precision)") (InputAction :type "InputAction Object Reference" :default "/Game/Core/Data/Input/Action/IA_Move.IA_Move"))
  (bind (_x _y) (`KismetMathLibrary.BreakVector2D` ActionValue))
  ;[0.02725 0.03125 0.02783 1 24] Передвижение игрока
  (:`Triggered`
    (`self.AddMovementInput` (`self.GetActorForwardVector`) _x)
    (`self.AddMovementInput` (`self.GetActorRightVector`) _y)))

(event `EnhancedInput|/Game/Core/Data/Input/Action/IA_Fire`
  (params (ActionValue :type Boolean) (ElapsedSeconds :type "Float (double-precision)") (TriggeredSeconds :type "Float (double-precision)") (InputAction :type "InputAction Object Reference" :default "/Game/Core/Data/Input/Action/IA_Fire.IA_Fire"))
  (bind _childactor (`ChildActorComponent.ChildActor` (`self.WeaponActor`)))
  ;[0.02725 0.03125 0.02783] Стрельба из оружия
  (:`Started`
    (message `/Game/Core/Interfaces/BPI_WeaponFireInterface.BPI_StartFire` _childactor))
  (:`Completed`
    (message `/Game/Core/Interfaces/BPI_WeaponFireInterface.BPI_StopFire` _childactor)))

(event `EnhancedInput|/Game/Core/Data/Input/Action/IA_Look`
  (params (ActionValue :type "Vector2D Structure") (ElapsedSeconds :type "Float (double-precision)") (TriggeredSeconds :type "Float (double-precision)") (InputAction :type "InputAction Object Reference" :default "/Game/Core/Data/Input/Action/IA_Look.IA_Look"))
  (bind (_x _y) (`KismetMathLibrary.BreakVector2D` ActionValue))
  ;[0.02725 0.03125 0.02783 1 24] Вращение камеры игрока
  (:`Triggered`
    (`self.AddControllerYawInput` _x)
    (`self.AddControllerPitchInput` _y)))

(event `EnhancedInput|/Game/Core/Data/Input/Action/IA_FireMode`
  (params (ActionValue :type Boolean) (ElapsedSeconds :type "Float (double-precision)") (TriggeredSeconds :type "Float (double-precision)") (InputAction :type "InputAction Object Reference" :default "/Game/Core/Data/Input/Action/IA_FireMode.IA_FireMode"))
  ;[0.02725 0.03125 0.02783 1 24] Смена режима огня
  (:`Started`
    (message `/Game/Core/Interfaces/BPI_FireMode.BPI_NextFireMode` (`ChildActorComponent.ChildActor` (`self.WeaponActor`)))))

(event `EnhancedInput|/Game/Core/Data/Input/Action/IA_Reload`
  (params (ActionValue :type Boolean) (ElapsedSeconds :type "Float (double-precision)") (TriggeredSeconds :type "Float (double-precision)") (InputAction :type "InputAction Object Reference" :default "/Game/Core/Data/Input/Action/IA_Reload.IA_Reload"))
  ;[0.02725 0.03125 0.02783 1 24] Перезарядка оружия
  (:`Started`
    (message `/Game/Core/Interfaces/BPI_ReloadInterface.BPI_StartReload` (`ChildActorComponent.ChildActor` (`self.WeaponActor`)))))

(fn `ReceiveBeginPlay`)

(fn `ReceivePossessed`
  (params (NewController :type "Controller Object Reference"))
  ; Инициализация управления персонажем
  (bind _asplayer_controller (cast `PlayerController` NewController))
  (`EnhancedInputSubsystemInterface.AddMappingContext` (pcsubsystem `EnhancedInputLocalPlayerSubsystem` _asplayer_controller) "/Game/Core/Data/Input/IMC/IMC_Default.IMC_Default" 0 (struct)))

(fn `UserConstructionScript`)