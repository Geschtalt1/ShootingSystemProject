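; Shooting component that lets its owning actor fire along the player's camera view.
; It overrides the parent's fire hooks, taking origin and direction from player 0's camera manager.
; On begin play it caches the owner's reload component and blocks firing while that component is reloading, on top of the parent's fire check.
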(fn `CanFireInternal`
  (returns (ReturnValue :type Boolean))
  (bind _returnvalue (`parent.CanFireInternal`))
  (return (and _returnvalue (not (`ReloadComponent.IsReloading` (`self.ReloadComponent`))))))

(fn `GetFireDirectionInternal`
  (returns (ReturnValue :type "Vector Structure"))
  (return (`Actor.GetActorForwardVector` (`GameplayStatics.GetPlayerCameraManager` 0))))

(fn `GetFireLocationInternal`
  (returns (ReturnValue :type "Vector Structure"))
  (return (`Actor.K2_GetActorLocation` (`GameplayStatics.GetPlayerCameraManager` 0))))

(fn `ReceiveBeginPlay`
  (set `self.ReloadComponent` (`Actor.GetComponentByClass` (`self.GetOwner`) "/Script/ShootingSystem.ReloadComponent")))