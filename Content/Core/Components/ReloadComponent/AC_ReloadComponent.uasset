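; AC_ReloadComponent is a Blueprint reload component that links reloading to the owning actor's ShootingComponent, which it caches on BeginPlay.
; Reload is allowed only when the parent check passes, reserve ammo remains and the magazine is not full.
; Starting a reload stops firing, and a successful reload refreshes the magazine through the ShootingComponent.
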(fn `CanReloadInternal`
  (returns (ReturnValue :type Boolean))
  (bind _returnvalue (`parent.CanReloadInternal`))
  (return (and _returnvalue (> (`.Total` (break `AmmoInfo` (`ShootingComponent.GetAmmo` (`self.ShootingComponent`)))) 0) (not (`ShootingComponent.IsFullAmmoInMagazine` (`self.ShootingComponent`))))))

(fn `ReceiveBeginPlay`
  (set `self.ShootingComponent` (`Actor.GetComponentByClass` (`self.GetOwner`) "/Script/ShootingSystem.ShootingComponent")))

(fn `ReceiveReloading`
  (params (bSuccessfully :type Boolean))
  (bind _shootingcomponent (`self.ShootingComponent`))
  ; Обновляем стак патронов в ShootingComponent когда перезарядка завершилась успешно
  (if bSuccessfully
    (`/Engine/EditorBlueprintResources/StandardMacros.IsValid` _shootingcomponent
      (:`Is Valid`
        (`ShootingComponent.RefreshMagazine` _shootingcomponent)))))

(fn `ReceiveStartReload`
  (bind _shootingcomponent (`self.ShootingComponent`)
    (:`then`
      (`ShootingComponent.FinishFire` _shootingcomponent))
    (:`else`)))