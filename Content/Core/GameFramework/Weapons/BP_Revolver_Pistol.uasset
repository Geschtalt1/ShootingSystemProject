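; Revolver pistol weapon Blueprint that exposes fire, reload and fire-mode switching through interface events.
; It delegates to shooting and reload components, both given the weapon mesh on BeginPlay, with the object pool component set as the shooting component's projectile pool.
; Stop-fire finishes shooting only in Auto fire mode.
; Target hits from bullets or line traces go to the hit impact component for surface impact handling.
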(event `/Game/Core/Interfaces/BPI_WeaponFireInterface.BPI_StopFire`
  ;[0.015 0.015 0.015 1 24] Останавливает стрельбу из пистолета
  (switch `EFireMode` (`ShootingComponent.GetFireMode` (`self.ShootingComponent`))
    (:`FM_Auto`
      (`ShootingComponent.FinishFire` (`self.ShootingComponent`)))))

(event `self.ReceiveBeginPlay`
  ;[0.015 0.015 0.015 1 24] Event BeginPlay
  (`ShootingComponent.SetMesh` (`self.ShootingComponent`) (`self.Mesh`))
  (`ShootingComponent.SetProjectilePoolManager` (`self.ShootingComponent`) (`self.ObjectPoolComponent`) true)
  (`ReloadComponent.SetMesh` (`self.ReloadComponent`) (`self.Mesh`)))

(event `/Game/Core/Interfaces/BPI_WeaponFireInterface.BPI_StartFire`
  ;[0.015 0.015 0.015 1 24] Начинает стрельбу из пистолета
  (`ShootingComponent.StartFire` (`self.ShootingComponent`)))

(event `/Game/Core/Interfaces/BPI_ReloadInterface.BPI_StartReload`
  ;[0.015 0.015 0.015 1 24] Запускает процесс перезарядки
  (`ReloadComponent.StartReload` (`self.ReloadComponent`)))

(event `/Game/Core/Interfaces/BPI_FireMode.BPI_NextFireMode`
  ;[0.015 0.015 0.015 1 24] Смена режима огня
  (`ShootingComponent.NextFireMode` (`self.ShootingComponent`)))

(event `self.ShootingComponent.OnTargetHit`
  (params (HitActor :type "Actor Object Reference") (DamageAmount :type "Float (single-precision)") (HitInfo :type "HitResult Structure (by ref)") (SurfaceTag :type "GameplayTag Structure"))
  ;[0.015 0.015 0.015 1 24] Обрабатываем попадание по поверхности когда пуля или лайнтрейс достиг поверхности
  (`HitImpactComponent.HandleImpact` (`self.HitImpactComponent`) (make `HitImpactParams` HitInfo)))

(fn `UserConstructionScript`)