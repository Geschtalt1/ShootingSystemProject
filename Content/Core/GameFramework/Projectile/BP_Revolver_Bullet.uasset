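; Pooled revolver bullet projectile that reports its impacts back to the weapon that fired it.
; Leaving the pool reactivates projectile movement along the actor's forward vector at fixed speed; returning deactivates it.
; On mesh hit, DefineSurface rebuilds the hit result with the physical material from a zero-length sphere trace at the bullet's location.
; That result goes to the ShootingComponent on the pool manager's owner, then the bullet returns to the pool.
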(event `self.PoolableComponent.OnUsedFromPool`
  ; Активация пули когда она берется из пула у огнестрела для стрельбы
  (`MovementComponent.SetUpdatedComponent` (`self.ProjectileComponent`) (`self.RootComponent`))
  (`ActorComponent.Activate` (`self.ProjectileComponent`) true)
  (set `MovementComponent.Velocity` (* (`self.GetActorForwardVector`) 15000.0) (`self.ProjectileComponent`))
  (`SceneComponent.SetRelativeScale3D` (`self.ProjectileMesh`) (5.0 5.0 5.0)))

(event `self.PoolableComponent.OnReturnedToPool`
  ; Деактивируем ProjectileMovement когда пуля вернулась в пулл
  (`ActorComponent.Deactivate` (`self.ProjectileComponent`)))

(event `self.ProjectileMesh.OnComponentHit`
  (params (HitComponent :type "PrimitiveComponent Object Reference") (OtherActor :type "Actor Object Reference") (OtherComp :type "PrimitiveComponent Object Reference") (NormalImpulse :type "Vector Structure") (Hit :type "HitResult Structure (by ref)"))
  (bind _returnvalue (`PoolableComponent.GetPoolManager` (`self.PoolableComponent`)))
  (bind _returnvalue_2 (`ActorComponent.GetOwner` _returnvalue))
  ; Обрабатываем попадание пули
  (`/Engine/EditorBlueprintResources/StandardMacros.IsValid` _returnvalue
    (:`Is Valid`
      (`/Engine/EditorBlueprintResources/StandardMacros.IsValid` _returnvalue_2
        (:`Is Valid`
          (`ShootingComponent.Notify_HandleHit` (`self.GetComponentByClass` _returnvalue_2 "/Script/ShootingSystem.ShootingComponent") (`self.DefineSurface` Hit))
          (`PoolableComponent.ReturnToPool` (`self.PoolableComponent`)))))))

(fn `DefineSurface`
  (params (Hit :type "HitResult Structure (by ref)"))
  (returns (ReturnValue :type "HitResult Structure"))
  (bind (_bblockinghit _binitialoverlap _time _distance _location _impactpoint _normal _impactnormal _physmat _hitactor _hitcomponent _hitbonename _bonename _hititem _elementindex _faceindex _tracestart _traceend) (`GameplayStatics.BreakHitResult` Hit))
  (bind _returnvalue (`SceneComponent.K2_GetComponentLocation` (`self.ProjectileMesh`)))
  (if _bblockinghit
    (bind _outhit (`KismetSystemLibrary.SphereTraceSingle` :`Start` _returnvalue :`End` _returnvalue :`Radius` (`self.CheckRadius`) :`TraceChannel` "TraceTypeQuery1" :`DrawDebugType` (`self.DebugTrace`)))
    (return (`GameplayStatics.MakeHitResult` _bblockinghit _binitialoverlap _time _distance _location _impactpoint _normal _impactnormal (`.PhysMat` (`GameplayStatics.BreakHitResult` _outhit)) _hitactor _hitcomponent _hitbonename _bonename _hititem _elementindex _faceindex _tracestart _traceend))))

(fn `UserConstructionScript`)