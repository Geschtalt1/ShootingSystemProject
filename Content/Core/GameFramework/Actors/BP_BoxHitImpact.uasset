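; BP_BoxHitImpact is a labeled box actor with a configurable surface, apparently for showing or testing hit impacts per surface type.
; The construction script applies the Material variable to the Cube and writes SurfaceName to four text renders.
; On BeginPlay it sets PhysMaterial as the Cube's physical material override, so the physical surface is applied only at runtime.
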(fn `ReceiveBeginPlay`
  (`PrimitiveComponent.SetPhysMaterialOverride` (`self.Cube`) (`self.Phys Material`)))

(fn `UserConstructionScript`
  (`PrimitiveComponent.SetMaterial` (`self.Cube`) 0 (`self.Material`))
  (`TextRenderComponent.K2_SetText` (`self.TextRender`) (`self.SurfaceName`))
  (`TextRenderComponent.K2_SetText` (`self.TextRender1`) (`self.SurfaceName`))
  (`TextRenderComponent.K2_SetText` (`self.TextRender2`) (`self.SurfaceName`))
  (`TextRenderComponent.K2_SetText` (`self.TextRender3`) (`self.SurfaceName`)))